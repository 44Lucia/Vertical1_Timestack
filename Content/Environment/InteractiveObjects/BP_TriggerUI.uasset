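; BP_TriggerUI is a trigger volume that shows an info panel on the first-person character's UI while the player stands inside it.
; On begin overlap it activates the panel on the character's UI, passing its RowName to select the entry.
; On end overlap it waits briefly, plays the UI's ClosePanel animation, then deactivates the panel after a second delay.
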(event `self.TriggerBox.OnComponentBeginOverlap`
  (params (OverlappedComponent :type "PrimitiveComponent Object Reference") (OtherActor :type "Actor Object Reference") (OtherComp :type "PrimitiveComponent Object Reference") (OtherBodyIndex :type Integer) (bFromSweep :type Boolean) (SweepResult :type "HitResult Structure (by ref)"))
  (bind _asbp_first_person_character (cast `/Game/Character/Blueprints/FirstPerson/BP_FirstPersonCharacter` OtherActor))
  (`/Game/Character/Blueprints/FirstPerson/MainUI.SetActivePanel` (`/Game/Character/Blueprints/FirstPerson/BP_FirstPersonCharacter.UI` _asbp_first_person_character) true (`self.RowName`)))

(event `self.TriggerBox.OnComponentEndOverlap`
  (params (OverlappedComponent :type "PrimitiveComponent Object Reference") (OtherActor :type "Actor Object Reference") (OtherComp :type "PrimitiveComponent Object Reference") (OtherBodyIndex :type Integer))
  (bind _asbp_first_person_character (cast `/Game/Character/Blueprints/FirstPerson/BP_FirstPersonCharacter` OtherActor))
  (`KismetSystemLibrary.Delay` 1.0)
  (bind _ui (`/Game/Character/Blueprints/FirstPerson/BP_FirstPersonCharacter.UI` _asbp_first_person_character))
  (`UserWidget.PlayAnimation` _ui (`/Game/Character/Blueprints/FirstPerson/MainUI.ClosePanel` _ui) 0.0 1 "Forward" 1.0 false)
  (`KismetSystemLibrary.Delay` 2.0)
  (`/Game/Character/Blueprints/FirstPerson/MainUI.SetActivePanel` _ui false (`self.RowName`)))

(fn `UserConstructionScript`)
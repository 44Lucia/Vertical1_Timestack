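; BP_SequenceButton is an interactable button that steps through its Actionables array in a looping sequence.
; Each interaction activates the next actionable and plays the Actionate timeline, which rotates the LadoLow component around its roll axis.
; In parallel, a delay set by DelayBetweenActivation runs before the current actionable deactivates and the index advances with wraparound, so the two briefly overlap.
; ResetState returns only the index to the first entry.
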(event `/Game/Environment/InteractiveObjects/I_PlayerInteractable.Interact`
  (params (Player :type "Character Object Reference"))
  (`|ExecutionSequence`
    (:`then_0`
      ; Activate next actionable
      (`/Game/Environment/InteractiveObjects/I_Actionable.Activate` (`|GetArrayItem` (`self.Actionables`) (mod (+ (`self.CurrentInteractableIndex`) 1) (`KismetArrayLibrary.Array_Length` (`self.Actionables`)))))
      (bind (_direction _angle) (`Timeline|Actionate` :!via `PlayFromStart`)
        (:`Update`
          (`SceneComponent.K2_SetRelativeRotation` (`self.Lado_low`) (`KismetMathLibrary.MakeRotator` _angle) false false))))
    (:`then_1`
      ; Deactivate current actionable
      (`KismetSystemLibrary.Delay` (`self.DelayBetweenActivation`))
      (`/Game/Environment/InteractiveObjects/I_Actionable.Deactivate` (`|GetArrayItem` (`self.Actionables`) (`self.CurrentInteractableIndex`)))
      (set `self.CurrentInteractableIndex` (mod (+ (`self.CurrentInteractableIndex`) 1) (`KismetArrayLibrary.Array_Length` (`self.Actionables`)))))))

(event `/Game/Environment/InteractiveObjects/I_PlayerInteractable.ResetState`
  (set `self.CurrentInteractableIndex` 0))

(fn `UserConstructionScript`)
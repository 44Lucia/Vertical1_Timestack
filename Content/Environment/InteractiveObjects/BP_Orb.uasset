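; BP_Orb is a collectible orb whose OrbColor picks its Niagara effect in the Construction Script.
; When the player overlaps its trigger, it plays a sound, optionally grants that color's power, flags HasOrb on the level manager and updates the UI.
; An overlapping BP_AlexClone only deactivates the orb.
; SetActive toggles trigger collision and effect visibility instead of destroying the actor.
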(event `self.ReceiveBeginPlay`
  (bind _returnvalue (`GameplayStatics.GetActorOfClass` "/Game/Character/Blueprints/LevelManagement/BP_LevelManager.BP_LevelManager_C"))
  (set `self.LevelManager` _returnvalue)
  (bind _asbp_first_person_character (cast `/Game/Character/Blueprints/FirstPerson/BP_FirstPersonCharacter` (`GameplayStatics.GetPlayerCharacter` 0)))
  (set `self.Player` _asbp_first_person_character))

(event `self.Trigger.OnComponentBeginOverlap`
  (params (OverlappedComponent :type "PrimitiveComponent Object Reference") (OtherActor :type "Actor Object Reference") (OtherComp :type "PrimitiveComponent Object Reference") (OtherBodyIndex :type Integer) (bFromSweep :type Boolean) (SweepResult :type "HitResult Structure (by ref)"))
  (`|ExecutionSequence`
    (:`then_0`
      (bind _asbp_first_person_character (cast `/Game/Character/Blueprints/FirstPerson/BP_FirstPersonCharacter` OtherActor))
      (`GameplayStatics.PlaySoundAtLocation` "/Game/Sounds/Ability/CollectOrb.CollectOrb" (`self.K2_GetActorLocation`) (struct) 1.0 1.0 0.0 null null null null)
      (`|ExecutionSequence`
        (:`then_0`
          (if (`self.ActivateAbility`)
            (`/Game/Character/Blueprints/FirstPerson/BP_FirstPersonCharacter.SetActivePower` _asbp_first_person_character (`self.OrbColor`))))
        (:`then_1`
          (set `/Game/Character/Blueprints/LevelManagement/BP_LevelManager.HasOrb` true (`self.LevelManager`))
          (`self.SetActive` false)
          (`/Game/Character/Blueprints/FirstPerson/MainUI.GetOrb` (`/Game/Character/Blueprints/FirstPerson/BP_FirstPersonCharacter.UI` (`self.Player`))))))
    (:`then_1`
      (cast `/Game/Character/Blueprints/Clone/BP_AlexClone` OtherActor)
      (`self.SetActive` false))))

(fn `SetActive`
  (params (NewState :type Boolean))
  (if NewState
    (`PrimitiveComponent.SetCollisionEnabled` (`self.Trigger`) "QueryAndPhysics")
    (`SceneComponent.SetHiddenInGame` (`self.Niagara`) false true)
    (else
      (`PrimitiveComponent.SetCollisionEnabled` (`self.Trigger`) "NoCollision")
      (`SceneComponent.SetHiddenInGame` (`self.Niagara`) true true))))

(fn `UserConstructionScript`
  (bind _niagara (`self.Niagara`))
  (switch `/Game/Character/Blueprints/LevelManagement/E_AbilityType` (`self.OrbColor`)
    (:`NewEnumerator0`
      (`NiagaraComponent.SetAsset` _niagara "/Game/Environment/Orbe/Orbe_Neutro.Orbe_Neutro" true))
    (:`NewEnumerator1`
      (`NiagaraComponent.SetAsset` _niagara "/Game/Environment/Orbe/Orbe_Rojo.Orbe_Rojo" true))
    (:`NewEnumerator2`
      (`NiagaraComponent.SetAsset` _niagara "/Game/Environment/Orbe/Orbe_Verde.Orbe_Verde" true))
    (:`NewEnumerator3`
      (`NiagaraComponent.SetAsset` _niagara "/Game/Environment/Orbe/Orbe_Azul.Orbe_Azul" true))))
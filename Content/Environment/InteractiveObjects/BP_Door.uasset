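; BP_Door is an interactive environment door that opens on Activate and closes on Deactivate, in a big or small variant.
; The construction script uses IsBigDoor to show one mesh and disable collision on the other.
; Timelines lerp the big door upward or the small door by LocationSmallDoor, and reverse to close.
; ResetState rewinds both timelines, then resets the big door's location or the small door's rotation.
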(event `/Game/Environment/InteractiveObjects/I_Actionable.Activate`
  (bind _returnvalue (`SceneComponent.K2_GetComponentLocation` (`self.DefaultSceneRoot`)))
  (bind _returnvalue_2 (`SceneComponent.K2_GetComponentLocation` (`self.DefaultSceneRoot`)))
  (if (`self.IsBigDoor`)
    (bind (_direction _alpha) (`Timeline|Big Door Open` :!label _label)
      (:`Update`
        (`SceneComponent.K2_SetWorldLocation` (`self.BigDoor`) (`KismetMathLibrary.VLerp` _returnvalue_2 (+ _returnvalue_2 (0.0 0.0 400.0)) _alpha) false false)))
    (else
      (bind (_direction_2 _alpha_2) (`Timeline|Small Door Open` :!label _label_2)
        (:`Update`
          (`SceneComponent.K2_SetWorldLocation` (`self.SmallDoor`) (`KismetMathLibrary.VLerp` _returnvalue (+ _returnvalue (`self.LocationSmallDoor`)) _alpha_2) false false))))))

(event `/Game/Environment/InteractiveObjects/I_Actionable.Deactivate`
  (if (`self.IsBigDoor`)
    (goto _label :!via `Reverse`)
    (else
      (goto _label_2 :!via `Reverse`))))

(event `/Game/Environment/InteractiveObjects/I_Actionable.ResetState`
  (`|ExecutionSequence`
    (:`then_0`
      (goto _label :!via `PlayFromStart`))
    (:`then_1`
      (goto _label :!via `Stop`))
    (:`then_2`
      (goto _label_2 :!via `PlayFromStart`))
    (:`then_3`
      (goto _label_2 :!via `Stop`))
    (:`then_4`
      (if (`self.IsBigDoor`)
        (`SceneComponent.K2_SetRelativeLocation` (`self.BigDoor`) (0.0 0.0 0.0) false true)
        (else
          (`SceneComponent.K2_SetRelativeRotation` (`self.SmallDoor`) (struct :`Yaw` -90.0 :`Roll` 90.0) false false))))))

(fn `UserConstructionScript`
  (bind _isbigdoor (`self.IsBigDoor`))
  (`SceneComponent.SetVisibility` (`self.BigDoor`) _isbigdoor false)
  (`SceneComponent.SetVisibility` (`self.SmallDoor`) (not _isbigdoor) false)
  (if (`self.IsBigDoor`)
    (`PrimitiveComponent.SetCollisionEnabled` (`self.SmallDoor`) "NoCollision")
    (else
      (`PrimitiveComponent.SetCollisionEnabled` (`self.BigDoor`) "NoCollision"))))
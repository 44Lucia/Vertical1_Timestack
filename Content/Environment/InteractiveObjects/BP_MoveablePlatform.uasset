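; BP_MoveablePlatform is an interactive platform that moves between its placed position and an end point.
; On BeginPlay it caches the start location and converts the EndPos offset from local to world space.
; Activate plays a timeline that lerps the actor between both points without sweeping, and Deactivate reverses it.
; ResetState teleports it back to the start without touching the timeline.
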(event `self.ReceiveBeginPlay`
  ; BeginPlay
  (set `self.StartPos` (`self.K2_GetActorLocation`))
  (set `self.EndPosWorld` (`KismetMathLibrary.TransformLocation` (`self.GetTransform`) (`self.EndPos`))))

(event `/Game/Environment/InteractiveObjects/I_Actionable.Activate`
  (bind (_direction _alpha) (`Timeline|Timeline` :!label _label)
    (:`Update`
      (`self.K2_SetActorLocation` (`KismetMathLibrary.VLerp` (`self.StartPos`) (`self.EndPosWorld`) _alpha)))))

(event `/Game/Environment/InteractiveObjects/I_Actionable.Deactivate`
  (goto _label :!via `Reverse`))

(event `/Game/Environment/InteractiveObjects/I_Actionable.ResetState`
  (`self.K2_SetActorLocation` (`self.StartPos`) false true))

(fn `UserConstructionScript`)
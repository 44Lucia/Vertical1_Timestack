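; BP_PickupBox is an interactive physics box that the first-person player can grab and release.
; It caches a reference to BP_FirstPersonCharacter on BeginPlay.
; Interact adds velocity to the cube along the camera's forward vector, then calls GrabObject on the character.
; EndInteract calls the character's ReleaseObject, leaving the hold logic to the character.
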(event `self.ReceiveBeginPlay`
  (bind _returnvalue (`GameplayStatics.GetActorOfClass` "/Game/FirstPerson/Blueprints/FirstPerson/BP_FirstPersonCharacter.BP_FirstPersonCharacter_C"))
  (set `self.PlayerRef` _returnvalue))

(event `/Game/Environment/InteractiveObjects/I_Interactable.Interact`
  (params (Player :type "Character Object Reference"))
  (`PrimitiveComponent.SetPhysicsLinearVelocity` (`self.Cube`) (* (`KismetMathLibrary.GetForwardVector` (`PlayerCameraManager.GetCameraRotation` (`PlayerController.PlayerCameraManager` (`GameplayStatics.GetPlayerController` 0)))) 500.0) true "None")
  (`/Game/FirstPerson/Blueprints/FirstPerson/BP_FirstPersonCharacter.GrabObject` (`self.PlayerRef`)))

(event `/Game/Environment/InteractiveObjects/I_Interactable.EndInteract`
  (`/Game/FirstPerson/Blueprints/FirstPerson/BP_FirstPersonCharacter.ReleaseObject` (`self.PlayerRef`) false))

(fn `UserConstructionScript`)
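; BP_Cube is an interactive cube the first-person character pushes, pulls and slides while interacting with it.
; Overlaps on the Fwd component gate interaction, and Interact toggles the grab state, cube physics simulation and a reduced player walk speed.
; While grabbed and in range, Tick reads the character's movement axes and calls Speed/Direction, which nudges the mesh along its own right/forward vectors using VInterpTo without sweep.
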(event `self.ReceiveBeginPlay`
  (bind _returnvalue (`GameplayStatics.GetActorOfClass` "/Game/FirstPerson/Blueprints/FirstPerson/BP_FirstPersonCharacter.BP_FirstPersonCharacter_C"))
  (set `self.characterREF` _returnvalue))

(event `/Game/Environment/InteractiveObjects/I_PlayerInteractable.Interact`
  (params (Player :type "Character Object Reference"))
  (bind _characterref (`self.characterREF`))
  (bind _characterref_2 (`self.characterREF`))
  (bind _sm_cube (`self.SM_Cube`))
  (bind _charactermovement (`Character.CharacterMovement` _characterref_2))
  (if (`/Game/FirstPerson/Blueprints/FirstPerson/BP_FirstPersonCharacter.canInteractBox` _characterref)
    (if (`/Game/FirstPerson/Blueprints/FirstPerson/BP_FirstPersonCharacter.isInteractingBox` _characterref)
      (set `/Game/FirstPerson/Blueprints/FirstPerson/BP_FirstPersonCharacter.isInteractingBox` false _characterref_2)
      (set `CharacterMovementComponent.MaxWalkSpeed` 600.0 _charactermovement)
      (`PrimitiveComponent.SetSimulatePhysics` _sm_cube false)
      (else
        (set `/Game/FirstPerson/Blueprints/FirstPerson/BP_FirstPersonCharacter.isInteractingBox` true _characterref_2)
        (set `CharacterMovementComponent.MaxWalkSpeed` 60.0 _charactermovement)
        (`PrimitiveComponent.SetSimulatePhysics` _sm_cube true)))))

(event `self.Fwd.OnComponentBeginOverlap`
  (params (OverlappedComponent :type "PrimitiveComponent Object Reference") (OtherActor :type "Actor Object Reference") (OtherComp :type "PrimitiveComponent Object Reference") (OtherBodyIndex :type Integer) (bFromSweep :type Boolean) (SweepResult :type "HitResult Structure (by ref)"))
  (`KismetSystemLibrary.PrintString` "CharacterCanInteract" true true (struct :`G` 1.0 :`B` 0.07428 :`A` 1.0) 2.0 "432342")
  (set `/Game/FirstPerson/Blueprints/FirstPerson/BP_FirstPersonCharacter.canInteractBox` true (`self.characterREF`)))

(event `self.Fwd.OnComponentEndOverlap`
  (params (OverlappedComponent :type "PrimitiveComponent Object Reference") (OtherActor :type "Actor Object Reference") (OtherComp :type "PrimitiveComponent Object Reference") (OtherBodyIndex :type Integer))
  (`KismetSystemLibrary.PrintString` "CharacterCantInteract" true true (struct :`R` 1.0 :`B` 0.027276 :`A` 1.0) 2.0 "3423423423")
  (set `/Game/FirstPerson/Blueprints/FirstPerson/BP_FirstPersonCharacter.canInteractBox` false (`self.characterREF`)))

(event `self.ReceiveTick`
  (params (DeltaSeconds :type "Float (single-precision)"))
  (bind _characterref (`self.characterREF`))
  (bind _characterref_2 (`self.characterREF`))
  (bind _forwardbackwardsaxis (`/Game/FirstPerson/Blueprints/FirstPerson/BP_FirstPersonCharacter.forwardBackwardsAxis` _characterref_2))
  (bind _rightleftaxis (`/Game/FirstPerson/Blueprints/FirstPerson/BP_FirstPersonCharacter.rightLeftAxis` _characterref_2))
  (if (`/Game/FirstPerson/Blueprints/FirstPerson/BP_FirstPersonCharacter.isInteractingBox` _characterref)
    (if (`/Game/FirstPerson/Blueprints/FirstPerson/BP_FirstPersonCharacter.canInteractBox` _characterref)
      (`|ExecutionSequence`
        (:`then_0`
          (if (== _forwardbackwardsaxis 0.0)
            (`KismetSystemLibrary.PrintString` "isNotMovingForward" true true (struct :`R` 1.0 :`G` 0.184643 :`A` 1.0) 2.0 "423423")
            (elif (>= _forwardbackwardsaxis 0.1)
              (`KismetSystemLibrary.PrintString` "isMovingForward" true true (struct :`G` 0.990949 :`B` 1.0 :`A` 1.0) 2.0 "4234235532")
              (`self.Speed/Direction` true 15.0)
              (else
                (`KismetSystemLibrary.PrintString` "isMovingBackwards" true true (struct :`G` 0.424486 :`B` 1.0 :`A` 1.0) 2.0 "543543346")
                (`self.Speed/Direction` true -15.0)))))
        (:`then_1`
          (if (== _rightleftaxis 0.0)
            (`KismetSystemLibrary.PrintString` "isNotMovingForward" true true (struct :`R` 1.0 :`G` 0.184643 :`A` 1.0) 2.0 "423423")
            (elif (>= _rightleftaxis 0.1)
              (`KismetSystemLibrary.PrintString` "isMovingRight" true true (struct :`G` 0.990949 :`B` 1.0 :`A` 1.0) 2.0 "4234235532")
              (`self.Speed/Direction` false -15.0)
              (else
                (`KismetSystemLibrary.PrintString` "isMovingLeft" true true (struct :`G` 0.424486 :`B` 1.0 :`A` 1.0) 2.0 "543543346")
                (`self.Speed/Direction` false 15.0)))))))))

(fn `UserConstructionScript`)
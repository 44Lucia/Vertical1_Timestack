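; BP_InputRecorder is an actor component that records move and look input as timestamped records.
; Enhanced Input actions cache the latest values, which Tick samples every frame while recording, and RecordEvent adds entries tagged with an event type.
; Starting clears old records and stores the owner's transform and real-time start; stopping disables component tick.
; BeginPlay starts recording automatically, marked as debug.
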(event `EnhancedInput|/Game/FirstPerson/Input/Actions/IA_Move`
  (params (ActionValue :type "Vector2D Structure") (ElapsedSeconds :type "Float (double-precision)") (TriggeredSeconds :type "Float (double-precision)") (InputAction :type "InputAction Object Reference" :default "/Game/FirstPerson/Input/Actions/IA_Move.IA_Move"))
  ; Input
  (:`Triggered`
    (set `self.CurrentMove` ActionValue)))

(event `EnhancedInput|/Game/FirstPerson/Input/Actions/IA_Look`
  (params (ActionValue :type "Vector2D Structure") (ElapsedSeconds :type "Float (double-precision)") (TriggeredSeconds :type "Float (double-precision)") (InputAction :type "InputAction Object Reference" :default "/Game/FirstPerson/Input/Actions/IA_Look.IA_Look"))
  ; Input
  (:`Triggered`
    (set `self.CurrentLookDelta` ActionValue)))

(event `StartRecording`
  ; Recording events
  (set `self.Recording?` true)
  (set `self.StartTime` (`GameplayStatics.GetRealTimeSeconds`))
  (set `self.StartTransform` (`Actor.GetTransform` (`self.GetOwner`)))
  (`KismetArrayLibrary.Array_Clear` (`self.Records`))
  (`self.SetComponentTickEnabled` true))

(event `self.ReceiveBeginPlay`
  ; Debug
  (`self.StartRecording`))

(event `StopRecording`
  ; Recording events
  (set `self.Recording?` false)
  (`self.SetComponentTickEnabled` false))

(event `self.ReceiveTick`
  (params (DeltaSeconds :type "Float (single-precision)"))
  (if (`self.Recording?`)
    (`KismetArrayLibrary.Array_Add` (`self.Records`) (make `/Game/InputRecorder/S_InputRecord` (- (`GameplayStatics.GetRealTimeSeconds`) (`self.StartTime`)) (`self.CurrentMove`) (`self.CurrentLookDelta`)))))

(event `RecordEvent`
  (params (EventType :type "/Game/InputRecorder/EInputEventType Enum" :default "NewEnumerator0"))
  (`KismetArrayLibrary.Array_Add` (`self.Records`) (make `/Game/InputRecorder/S_InputRecord` (- (`GameplayStatics.GetRealTimeSeconds`) (`self.StartTime`)) (`self.CurrentMove`) (`self.CurrentLookDelta`) EventType)))
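; BP_AbilityBase is a base Blueprint for character abilities, with an enable switch and a readiness check.
; TryActivate runs only when enabled and ready, clears IsReady and calls ActivateImpl, an empty hook presumably for child abilities.
; It then starts a Cooldown timer with no event shown bound and sets IsReady true immediately, without waiting.
; Spanish debug prints report activation, ready, cooldown and disabled states.
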(fn `ActivateImpl`)

(fn `SetEnabled`
  (params (isEnabled :type Boolean))
  (set `self.isEnabled` isEnabled))

(fn `TryActivate`
  (if (`self.isEnabled`)
    (if (`self.isReady`)
      (set `self.isReady` false)
      (`KismetSystemLibrary.PrintString` "Activando poder...")
      (`self.ActivateImpl`)
      (`KismetSystemLibrary.K2_SetTimerDelegate` :`Time` (`self.Cooldown`))
      (set `self.isReady` true)
      (`KismetSystemLibrary.PrintString` "Poder listo")
      (else
        (`KismetSystemLibrary.PrintString` "En cooldown")
        (return)))
    (else
      (`KismetSystemLibrary.PrintString` "Poder Desactivado")
      (return))))
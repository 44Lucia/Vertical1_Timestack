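; Trigger volume that shows and hides a text panel on the first-person character's UI, apparently for ability text.
; BeginPlay caches the BP_FirstPersonCharacter, and any overlap with the Box activates its UI panel with no row name, without filtering the overlapping actor.
; End overlap waits, plays the ClosePanel animation in reverse, then waits again before deactivating the panel.
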(event `self.ReceiveBeginPlay`
  (bind _returnvalue (`GameplayStatics.GetActorOfClass` "/Game/Character/Blueprints/FirstPerson/BP_FirstPersonCharacter.BP_FirstPersonCharacter_C"))
  (set `self.Character` _returnvalue))

(event `self.Box.OnComponentBeginOverlap`
  (params (OverlappedComponent :type "PrimitiveComponent Object Reference") (OtherActor :type "Actor Object Reference") (OtherComp :type "PrimitiveComponent Object Reference") (OtherBodyIndex :type Integer) (bFromSweep :type Boolean) (SweepResult :type "HitResult Structure (by ref)"))
  (`/Game/Character/Blueprints/FirstPerson/MainUI.SetActivePanel` (`/Game/Character/Blueprints/FirstPerson/BP_FirstPersonCharacter.UI` (`self.Character`)) true "None"))

(event `self.Box.OnComponentEndOverlap`
  (params (OverlappedComponent :type "PrimitiveComponent Object Reference") (OtherActor :type "Actor Object Reference") (OtherComp :type "PrimitiveComponent Object Reference") (OtherBodyIndex :type Integer))
  (bind _ui (`/Game/Character/Blueprints/FirstPerson/BP_FirstPersonCharacter.UI` (`self.Character`)))
  (`KismetSystemLibrary.Delay` 2.0)
  (`UserWidget.PlayAnimation` _ui (`/Game/Character/Blueprints/FirstPerson/MainUI.ClosePanel` _ui) 0.0 1 "Reverse" 1.0 false)
  (`KismetSystemLibrary.Delay` 2.0)
  (`/Game/Character/Blueprints/FirstPerson/MainUI.SetActivePanel` _ui false "None"))

(fn `UserConstructionScript`)
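; Push ability for the first-person character that slides a "Movable" actor along the camera's flattened forward direction, despite its pull-named variables and sound.
; On activation, FindVoidAhead supplies the actor, its target is offset from its location, physics and gravity are suspended if simulating, and a sound plays.
; Tick moves it with swept VInterpTo until within the stop distance, then restores any suspended physics with zero velocity.
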(event `self.ReceiveTick`
  (params (DeltaSeconds :type "Float (single-precision)"))
  (bind _returnvalue (`KismetMathLibrary.VInterpTo` (`Actor.K2_GetActorLocation` (`self.PulledActor`)) (`self.TargetLoc`) (`GameplayStatics.GetWorldDeltaSeconds`) (`self.InterpSpeed`)))
  (`parent.ReceiveTick` DeltaSeconds)
  (if (`self.isPulling`)
    (cast `/Game/Character/Blueprints/FirstPerson/BP_FirstPersonCharacter` (`self.GetOwner`))
    (`Actor.K2_SetActorLocation` (`self.PulledActor`) _returnvalue true false)
    (if (<= (`KismetMathLibrary.Vector_Distance` _returnvalue (`self.TargetLoc`)) (`self.StopDist`))
      (if (`self.havePhysics`)
        (bind _asprimitive_component (cast `PrimitiveComponent` (`Actor.RootComponent` (`self.PulledActor`))))
        (`/Engine/EditorBlueprintResources/StandardMacros.IsValid` _asprimitive_component
          (:`Is Valid`
            (`PrimitiveComponent.SetSimulatePhysics` _asprimitive_component true)
            (`PrimitiveComponent.SetEnableGravity` _asprimitive_component true)
            (`PrimitiveComponent.SetPhysicsLinearVelocity` _asprimitive_component (0.0 0.0 0.0) false "None")
            (set `self.havePhysics` false)
            (set `self.isPulling` false)))
        (else
          (set `self.havePhysics` false)
          (set `self.isPulling` false))))))

(fn `ActivateImpl`
  (`parent.ActivateImpl`)
  (bind _asbp_first_person_character (cast `/Game/Character/Blueprints/FirstPerson/BP_FirstPersonCharacter` (`self.GetOwner`)))
  (bind (_isvoid _hitresult _hitcomponents) (`/Game/Character/Blueprints/FirstPerson/BP_FirstPersonCharacter.FindVoidAhead` _asbp_first_person_character 1000.0 3000.0))
  (if _isvoid
    (`/Engine/EditorBlueprintResources/StandardMacros.IsValid` _hitresult
      (:`Is Valid`
        (`/Engine/EditorBlueprintResources/StandardMacros.IsValid` _hitcomponents
          (:`Is Valid`
            (if (`Actor.ActorHasTag` _hitresult "Movable")
              (`KismetSystemLibrary.PrintString` "OBJETO")
              (bind _output_get (set `self.PulledActor` _hitresult))
              (bind (_returnvalue_x _returnvalue_y) (`KismetMathLibrary.BreakVector` (`SceneComponent.GetForwardVector` (`/Game/Character/Blueprints/FirstPerson/BP_FirstPersonCharacter.FirstPersonCamera` _asbp_first_person_character))))
              (set `self.TargetLoc` (+ (`Actor.K2_GetActorLocation` (`self.PulledActor`)) (* (`KismetMathLibrary.Normal` (`KismetMathLibrary.MakeVector` _returnvalue_x _returnvalue_y 1e-05)) (`self.DistOffset`))))
              (bind _asprimitive_component (cast `PrimitiveComponent` (`Actor.RootComponent` _output_get)))
              (`/Engine/EditorBlueprintResources/StandardMacros.IsValid` _asprimitive_component
                (:`Is Valid`
                  (if (`SceneComponent.IsSimulatingPhysics` _asprimitive_component "None")
                    (`PrimitiveComponent.SetSimulatePhysics` _asprimitive_component false)
                    (`PrimitiveComponent.SetEnableGravity` _asprimitive_component false)
                    (`PrimitiveComponent.SetPhysicsLinearVelocity` _asprimitive_component (0.0 0.0 0.0) false "None")
                    (set `self.havePhysics` true)
                    (set `self.isPulling` true)
                    (bind _returnvalue (`Actor.K2_GetActorLocation` _output_get))
                    (`GameplayStatics.PlaySoundAtLocation` "/Game/Sounds/Ability/PullAbility.PullAbility" _returnvalue (struct) 1.0 1.0 0.0 null null null null)
                    (else
                      (set `self.havePhysics` false)
                      (set `self.isPulling` true)
                      (`GameplayStatics.PlaySoundAtLocation` "/Game/Sounds/Ability/PullAbility.PullAbility" _returnvalue (struct) 1.0 1.0 0.0 null null null null))))))))))))
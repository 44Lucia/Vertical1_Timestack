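; Pull ability for the first-person character that draws a "Movable"-tagged actor toward a point in front of the camera.
; On activation it takes the target from the character's FindVoidAhead check, suspends any physics simulation and plays a sound.
; Tick moves the actor with swept VInterpTo, following the camera horizontally while essentially keeping its own height.
; Within the stop distance, pulling ends and any suspended physics is restored with zero velocity.
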(event `self.ReceiveTick`
  (params (DeltaSeconds :type "Float (single-precision)"))
  (bind (_anchor_x _anchor_y) (`KismetMathLibrary.BreakVector` (`self.Anchor`)))
  (bind (_returnvalue_x _returnvalue_y _returnvalue_z) (`KismetMathLibrary.BreakVector` (`Actor.K2_GetActorLocation` (`self.PulledActor`))))
  (bind _returnvalue (`KismetMathLibrary.VInterpTo` (`Actor.K2_GetActorLocation` (`self.PulledActor`)) (`self.TargetLoc`) (`GameplayStatics.GetWorldDeltaSeconds`) (`self.InterpSpeed`)))
  (`parent.ReceiveTick` DeltaSeconds)
  (if (`self.isPulling`)
    (bind _asbp_first_person_character (cast `/Game/Character/Blueprints/FirstPerson/BP_FirstPersonCharacter` (`self.GetOwner`)))
    (bind _firstpersoncamera (`/Game/Character/Blueprints/FirstPerson/BP_FirstPersonCharacter.FirstPersonCamera` _asbp_first_person_character))
    (set `self.Anchor` (+ (+ (`SceneComponent.K2_GetComponentLocation` _firstpersoncamera) (* (`SceneComponent.GetForwardVector` _firstpersoncamera) (`self.DistOffset`))) (`self.UpOffset`)))
    (set `self.TargetLoc` (`KismetMathLibrary.MakeVector` _anchor_x _anchor_y (+ _returnvalue_z 0.001)))
    (`Actor.K2_SetActorLocation` (`self.PulledActor`) _returnvalue true false)
    (if (<= (`KismetMathLibrary.Vector_Distance` _returnvalue (`self.TargetLoc`)) (`self.StopDist`))
      (if (`self.havePhysics`)
        (bind _asprimitive_component (cast `PrimitiveComponent` (`Actor.RootComponent` (`self.PulledActor`))))
        (`/Engine/EditorBlueprintResources/StandardMacros.IsValid` _asprimitive_component
          (:`Is Valid`
            (`PrimitiveComponent.SetSimulatePhysics` _asprimitive_component true)
            (`PrimitiveComponent.SetEnableGravity` _asprimitive_component true)
            (`PrimitiveComponent.SetPhysicsLinearVelocity` _asprimitive_component (0.0 0.0 0.0) false "None")
            (set `self.havePhysics` false)
            (set `self.isPulling` false)))
        (else
          (set `self.havePhysics` false)
          (set `self.isPulling` false))))))

(fn `ActivateImpl`
  (`parent.ActivateImpl`)
  (bind _asbp_first_person_character (cast `/Game/Character/Blueprints/FirstPerson/BP_FirstPersonCharacter` (`self.GetOwner`)))
  (bind (_isvoid _hitresult _hitcomponents) (`/Game/Character/Blueprints/FirstPerson/BP_FirstPersonCharacter.FindVoidAhead` _asbp_first_person_character 2000.0 3000.0))
  (if _isvoid
    (`/Engine/EditorBlueprintResources/StandardMacros.IsValid` _hitresult
      (:`Is Valid`
        (`/Engine/EditorBlueprintResources/StandardMacros.IsValid` _hitcomponents
          (:`Is Valid`
            (if (`Actor.ActorHasTag` _hitresult "Movable")
              (`KismetSystemLibrary.PrintString` "OBJETO")
              (bind _output_get (set `self.PulledActor` _hitresult))
              (bind _asprimitive_component (cast `PrimitiveComponent` (`Actor.RootComponent` _output_get)))
              (`/Engine/EditorBlueprintResources/StandardMacros.IsValid` _asprimitive_component
                (:`Is Valid`
                  (if (`SceneComponent.IsSimulatingPhysics` _asprimitive_component "None")
                    (`PrimitiveComponent.SetSimulatePhysics` _asprimitive_component false)
                    (`PrimitiveComponent.SetEnableGravity` _asprimitive_component false)
                    (`PrimitiveComponent.SetPhysicsLinearVelocity` _asprimitive_component (0.0 0.0 0.0) false "None")
                    (set `self.havePhysics` true)
                    (set `self.isPulling` true)
                    (bind _returnvalue (`Actor.K2_GetActorLocation` _output_get))
                    (`GameplayStatics.PlaySoundAtLocation` "/Game/Sounds/Ability/PullPush.PullPush" _returnvalue (struct) 1.0 1.0 0.0 null null null null)
                    (else
                      (set `self.havePhysics` false)
                      (set `self.isPulling` true)
                      (`GameplayStatics.PlaySoundAtLocation` "/Game/Sounds/Ability/PullPush.PullPush" _returnvalue (struct) 1.0 1.0 0.0 null null null null))))))))))))
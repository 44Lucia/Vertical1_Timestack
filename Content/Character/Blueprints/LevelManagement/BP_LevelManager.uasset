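; Level manager for a timed clone-replay puzzle, stepping the player through color-coded ability iterations.
; First move, jump or click starts input recording, active clone playback and the countdown.
; At timeout, holding the orb switches the player to a clone and advances, or opens the next level after the last iteration; otherwise it retries.
; Each setup teleports and recolors the player and resets orbs, replays and interface-gathered level objects.
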(event `Key|LeftMouseButton`
  (params (Key :type "Key Structure"))
  ; Start input
  (:`Pressed`
    (if (not (`self.IsPlaying`)) :!label _label
      (set `self.IsPlaying` true)
      (`/Game/Character/Blueprints/Clone/AC_InputRecorder.StartRecording` (`/Game/Character/Blueprints/FirstPerson/BP_FirstPersonCharacter.AlexInputRecorder` (`self.Player`)))
      (for _array_element (`self.ActiveClones`)
        (`/Engine/EditorBlueprintResources/StandardMacros.IsValid` _array_element
          (:`Is Valid`
            (`/Game/Character/Blueprints/Clone/AC_InputPlayer.StartPlayback` (`/Game/Character/Blueprints/Clone/BP_AlexClone.AlexInputPlayer` _array_element))))))))

(event `EnhancedInput|/Game/Character/Input/Actions/IA_Move`
  (params (ActionValue :type "Vector2D Structure") (ElapsedSeconds :type "Float (double-precision)") (TriggeredSeconds :type "Float (double-precision)") (InputAction :type "InputAction Object Reference" :default "/Game/Character/Input/Actions/IA_Move.IA_Move"))
  ; Start input
  (:`Started`
    (goto _label)))

(event `EnhancedInput|/Game/Character/Input/Actions/IA_Jump`
  (params (ActionValue :type Boolean) (ElapsedSeconds :type "Float (double-precision)") (TriggeredSeconds :type "Float (double-precision)") (InputAction :type "InputAction Object Reference" :default "/Game/Character/Input/Actions/IA_Jump.IA_Jump"))
  ; Start input
  (:`Started`
    (goto _label)))

(event `ResetCurrentIteration`
  ; Reset iteration input
  (`/Game/Character/Blueprints/FirstPerson/MainUI.ResetLastOrb` (`/Game/Character/Blueprints/FirstPerson/BP_FirstPersonCharacter.UI` (`self.Player`)) :!label _label_2)
  (`self.SetupCurrentIteration`))

(event `self.ReceiveBeginPlay`
  ; BeginPlay
  (bind _asbp_first_person_character (cast `/Game/Character/Blueprints/FirstPerson/BP_FirstPersonCharacter` (`GameplayStatics.GetPlayerCharacter` 0)))
  (set `self.Player` _asbp_first_person_character)
  (`self.SetupCurrentIteration`)
  (`KismetSystemLibrary.Delay` 0.001)
  (`self.UpdateUIColor`)
  (`self.EnableInput` (`GameplayStatics.GetPlayerController` 0))
  (`|ExecutionSequence`
    (:`then_0`
      (bind _outactors (`GameplayStatics.GetAllActorsWithInterface` "/Game/Environment/InteractiveObjects/I_Actionable.I_Actionable_C"))
      (for _array_element _outactors
        (bind _asi_actionable (cast `/Game/Environment/InteractiveObjects/I_Actionable` _array_element))
        (`KismetArrayLibrary.Array_AddUnique` (`self.LevelActionables`) _asi_actionable)))
    (:`then_1`
      (bind _outactors_2 (`GameplayStatics.GetAllActorsWithInterface` "/Game/Environment/InteractiveObjects/I_PlayerInteractable.I_PlayerInteractable_C"))
      (for _array_element_2 _outactors_2
        (bind _asi_player_interactable (cast `/Game/Environment/InteractiveObjects/I_PlayerInteractable` _array_element_2))
        (`KismetArrayLibrary.Array_AddUnique` (`self.LevelPlayerInteractables`) _asi_player_interactable)))))

(event `EnhancedInput|/Game/Character/Input/Actions/IA_ResetIteration`
  (params (ActionValue :type Boolean) (ElapsedSeconds :type "Float (double-precision)") (TriggeredSeconds :type "Float (double-precision)") (InputAction :type "InputAction Object Reference" :default "/Game/Character/Input/Actions/IA_ResetIteration.IA_ResetIteration"))
  ; Reset iteration input
  (:`Triggered`
    (goto _label_2)))

(event `self.ReceiveTick`
  (params (DeltaSeconds :type "Float (single-precision)"))
  (bind (_output_abilitytype _output_spawnpoint _output_orb _output_totaltime) (break `/Game/Character/Blueprints/LevelManagement/S_LevelIteration` (`|GetArrayItem` (`self.LevelIterations`) (`self.CurrentIterationIndex`))))
  ; Event Tick
  (if (`self.IsPlaying`)
    (if (> (`self.RemainingTime`) 0.0)
      (set `self.RemainingTime` (`KismetMathLibrary.FClamp` (- (`self.RemainingTime`) DeltaSeconds) 0.0 _output_totaltime))
      (`self.UpdateUIBar`)
      (elif (`self.HasOrb`)
        (`self.ProcessNextIteration`)
        (else
          (`self.SetupCurrentIteration`)
          (`/Game/Character/Blueprints/FirstPerson/MainUI.ResetLastOrb` (`/Game/Character/Blueprints/FirstPerson/BP_FirstPersonCharacter.UI` (`self.Player`))))))))

(event `EnhancedInput|/Game/Character/Input/Actions/IA_ResetLevel`
  (params (ActionValue :type Boolean) (ElapsedSeconds :type "Float (double-precision)") (TriggeredSeconds :type "Float (double-precision)") (InputAction :type "InputAction Object Reference" :default "/Game/Character/Input/Actions/IA_ResetLevel.IA_ResetLevel"))
  ; Reset level input
  (:`Triggered`
    (if (not (`self.IsPlaying`))
      (set `self.CurrentIterationIndex` 0)
      (`|ExecutionSequence`
        (:`then_0`
          (`self.SetupCurrentIteration`)
          (`/Game/Character/Blueprints/FirstPerson/MainUI.ResetLastOrb` (`/Game/Character/Blueprints/FirstPerson/BP_FirstPersonCharacter.UI` (`self.Player`))))
        (:`then_1`
          (for _array_element (`self.ActiveClones`)
            (`/Engine/EditorBlueprintResources/StandardMacros.IsValid` _array_element
              (:`Is Valid`
                (`self.K2_DestroyActor` _array_element)))))))))

(fn `GetPlayerMaterials`
  (returns (Bottom :type "MaterialInstance Object Reference") (Top :type "MaterialInstance Object Reference"))
  (bind _output_abilitytype (break `/Game/Character/Blueprints/LevelManagement/S_LevelIteration` (`|GetArrayItem` (`self.LevelIterations`) (`self.CurrentIterationIndex`))))
  (switch `/Game/Character/Blueprints/LevelManagement/E_AbilityType` _output_abilitytype
    (:`NewEnumerator1`
      (return "/Game/Character/SpaceSuit/Materials/Red/MI_Red_PlayerBottom.MI_Red_PlayerBottom" "/Game/Character/SpaceSuit/Materials/Red/MI_Red_PlayerTop.MI_Red_PlayerTop"))
    (:`NewEnumerator2`
      (return "/Game/Character/SpaceSuit/Materials/Green/MI_Green_PlayerBottom.MI_Green_PlayerBottom" "/Game/Character/SpaceSuit/Materials/Green/MI_Green_PlayerTop.MI_Green_PlayerTop"))
    (:`NewEnumerator3`
      (return "/Game/Character/SpaceSuit/Materials/Blue/MI_Blue_PlayerBottom.MI_Blue_PlayerBottom" "/Game/Character/SpaceSuit/Materials/Blue/MI_Blue_PlayerTop.MI_Blue_PlayerTop"))))

(fn `ProcessNextIteration`
  (set `self.HasOrb` false)
  (if (>= (+ (`self.CurrentIterationIndex`) 1) (`KismetArrayLibrary.Array_Length` (`self.LevelIterations`)))
    (`KismetSystemLibrary.PrintString` "Win" true true (struct :`R` 0.35864 :`B` 1.0 :`A` 1.0))
    (set `self.IsPlaying` false)
    (`GameplayStatics.OpenLevel` (`self.NextLevel`))
    (else
      (`/Game/Character/Blueprints/FirstPerson/BP_FirstPersonCharacter.SwitchToClone` (`self.Player`))
      (`/Engine/EditorBlueprintResources/StandardMacros.IncrementInt` (`self.CurrentIterationIndex`)
        (:`  `
          (`self.SetupCurrentIteration`)
          (`self.UpdateUIColor`))))))

(fn `SetupCurrentIteration`
  (bind _player (`self.Player`))
  (bind (_output_abilitytype _output_spawnpoint _output_orb _output_totaltime) (break `/Game/Character/Blueprints/LevelManagement/S_LevelIteration` (`|GetArrayItem` (`self.LevelIterations`) (`self.CurrentIterationIndex`))))
  (bind _mesh (`Character.Mesh` (`self.Player`)))
  (bind (_returnvalue_location _returnvalue_rotation) (`KismetMathLibrary.BreakTransform` (`self.GetTransform` _output_spawnpoint)))
  (`|ExecutionSequence`
    (:`then_0`
      (`MovementComponent.StopMovementImmediately` (`Character.CharacterMovement` _player))
      (`self.K2_SetActorLocation` _player _returnvalue_location false true)
      (`Controller.SetControlRotation` (`Pawn.GetController` _player) _returnvalue_rotation)
      (`self.GetPlayerMaterials`)
      (bind (_bottom _top) (`self.GetPlayerMaterials`))
      (`PrimitiveComponent.SetMaterial` _mesh 0 _bottom)
      (`PrimitiveComponent.SetMaterial` _mesh 1 _top))
    (:`then_1`
      (`self.UpdateUIColor`))
    (:`then_2`
      (set `self.RemainingTime` _output_totaltime)
      (set `self.IsPlaying` false)
      (set `self.HasOrb` false)
      (`|ExecutionSequence`
        (:`then_0`
          (for _array_element (`self.LevelIterations`)
            (`/Game/Environment/InteractiveObjects/BP_Orb.SetActive` (`.Orb_3_AD9872634585D6FD57786290BEDA1CFB` (break `/Game/Character/Blueprints/LevelManagement/S_LevelIteration` _array_element)) true)))
        (:`then_1`
          (for _array_element_2 (`self.ActiveClones`)
            (`/Engine/EditorBlueprintResources/StandardMacros.IsValid` _array_element_2
              (:`Is Valid`
                (`/Game/Character/Blueprints/Clone/AC_InputPlayer.ResetReplay` (`/Game/Character/Blueprints/Clone/BP_AlexClone.AlexInputPlayer` _array_element_2))))))
        (:`then_2`
          (for _array_element_3 (`self.LevelActionables`)
            (`/Game/Environment/InteractiveObjects/I_Actionable.ResetState` _array_element_3)))
        (:`then_3`
          (for _array_element_4 (`self.LevelPlayerInteractables`)
            (`/Game/Environment/InteractiveObjects/I_PlayerInteractable.ResetState` _array_element_4)))
        (:`then_4`
          (`/Game/Character/Blueprints/Clone/AC_InputRecorder.StopRecording` (`/Game/Character/Blueprints/FirstPerson/BP_FirstPersonCharacter.AlexInputRecorder` (`self.Player`)))
          (`self.UpdateUIBar`))))))

(fn `UpdateUIBar`
  (bind (_output_abilitytype _output_spawnpoint _output_orb _output_totaltime) (break `/Game/Character/Blueprints/LevelManagement/S_LevelIteration` (`|GetArrayItem` (`self.LevelIterations`) (`self.CurrentIterationIndex`))))
  (bind _ui (`/Game/Character/Blueprints/FirstPerson/BP_FirstPersonCharacter.UI` (`self.Player`)))
  (`/Engine/EditorBlueprintResources/StandardMacros.IsValid` _ui
    (:`Is Valid`
      (`ProgressBar.SetPercent` (`/Game/Character/Blueprints/FirstPerson/MainUI.TimeBar` _ui) (`KismetMathLibrary.NormalizeToRange` (`self.RemainingTime`) 0.0 _output_totaltime)))))

(fn `UpdateUIColor`
  (bind _output_abilitytype (break `/Game/Character/Blueprints/LevelManagement/S_LevelIteration` (`|GetArrayItem` (`self.LevelIterations`) (`self.CurrentIterationIndex`))))
  (bind _ui (`/Game/Character/Blueprints/FirstPerson/BP_FirstPersonCharacter.UI` (`self.Player`)))
  (bind _timebar (`/Game/Character/Blueprints/FirstPerson/MainUI.TimeBar` _ui))
  (`self.UpdateUIBar`)
  (`/Engine/EditorBlueprintResources/StandardMacros.IsValid` _ui
    (:`Is Valid`
      (switch `/Game/Character/Blueprints/LevelManagement/E_AbilityType` _output_abilitytype
        (:`NewEnumerator1`
          (`ProgressBar.SetFillColorAndOpacity` _timebar (struct :`R` 1.0 :`A` 0.7)))
        (:`NewEnumerator2`
          (`ProgressBar.SetFillColorAndOpacity` _timebar (struct :`G` 1.0 :`A` 0.7)))
        (:`NewEnumerator3`
          (`ProgressBar.SetFillColorAndOpacity` _timebar (struct :`B` 1.0 :`A` 0.7)))))))

(fn `UserConstructionScript`
  (locals (NewLocalVar :type "/Game/Character/Blueprints/LevelManagement/S_LevelIteration Structure"))
  (for _array_element (`self.LevelIterations`)
    (switch `/Game/Character/Blueprints/LevelManagement/E_AbilityType` (break `/Game/Character/Blueprints/LevelManagement/S_LevelIteration` _array_element)
      (:`NewEnumerator1`
        (bind _capsule (`/Game/Character/Blueprints/LevelManagement/BP_IterationStartPoint.Capsule` (`.SpawnPoint_8_E0377D9A4930E27883E893982CF93FC0` (break `/Game/Character/Blueprints/LevelManagement/S_LevelIteration` _array_element))))
        (set `ShapeComponent.ShapeColor` (make `Color` 0 0 200 255) _capsule))
      (:`NewEnumerator2`
        (set `ShapeComponent.ShapeColor` (make `Color` 0 200 0 255) _capsule))
      (:`NewEnumerator3`
        (set `ShapeComponent.ShapeColor` (make `Color` 200 0 0 255) _capsule)))))
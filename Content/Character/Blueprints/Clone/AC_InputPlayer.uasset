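; Input playback component for BP_AlexClone that replays recorded move, look, jump and interact input on the clone.
; SetReplay loads the instruction arrays, and Tick advances a play clock that moves a separate index through each one.
; Movement holds values over time intervals, look interpolates between samples to set actor rotation, and jump and interact fire as timed press/release events.
; ResetReplay stops playback, clears state and teleports the clone to its start transform.
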(event `self.ReceiveBeginPlay`
  (bind _asbp_alex_clone (cast `/Game/Character/Blueprints/Clone/BP_AlexClone` (`self.GetOwner`)))
  (set `self.OwnerCharacter` _asbp_alex_clone))

(event `StartPlayback`
  (set `self.IsPlaying` true)
  (set `self.CurrentPlayTime` 0.0))

(event `SetReplay`
  (params (`Forward Instructions` :type "Array of /Game/Character/Blueprints/Clone/S_MoveInstruction Structure") (`Right Instructions` :type "Array of /Game/Character/Blueprints/Clone/S_MoveInstruction Structure") (`Look Samples` :type "Array of /Game/Character/Blueprints/Clone/S_LookSample Structure") (`Jump Instructions` :type "Array of /Game/Character/Blueprints/Clone/S_BoolInstruction Structure") (`Interact Instructions` :type "Array of /Game/Character/Blueprints/Clone/S_BoolInstruction Structure"))
  ; StartPlayback - Reset all variables
  (set `self.ForwardInstructions` `Forward Instructions`)
  (set `self.RightInstructions` `Right Instructions`)
  (set `self.LookSamples` `Look Samples`)
  (set `self.JumpInstructions` `Jump Instructions`)
  (set `self.InteractInstructions` `Interact Instructions`)
  (set `self.ForwardCurrentIndex` 0)
  (set `self.RightCurrentIndex` 0)
  (set `self.LookCurrentIndex` 0)
  (set `self.JumpCurrentIndex` 0)
  (set `self.InteractCurrentIndex` 0))

(event `self.ReceiveTick`
  (params (DeltaSeconds :type "Float (single-precision)"))
  ; Event tick
  (if (`self.IsPlaying`)
    (set `self.CurrentPlayTime` (+ DeltaSeconds (`self.CurrentPlayTime`)))
    (`self.ProcessLookInput`)
    (`self.ProcessForwardInput`)
    (`self.ProcessRightInput`)
    (`self.ProcessJumpInput`)
    (`self.ProcessInteractInput`)))

(fn `ProcessForwardInput`
  (bind _currentplaytime (`self.CurrentPlayTime`))
  (bind _ownercharacter (`self.OwnerCharacter`))
  (bind (_output_starttime _output_endtime _output_value) (break `/Game/Character/Blueprints/Clone/S_MoveInstruction` (`|GetArrayItem` (`self.ForwardInstructions`) (`self.ForwardCurrentIndex`))))
  (`|ExecutionSequence`
    (:`then_0`
      (if (< (`self.ForwardCurrentIndex`) (`KismetArrayLibrary.Array_Length` (`self.ForwardInstructions`))) :!label _label
        (if (> _currentplaytime _output_endtime)
          (`/Engine/EditorBlueprintResources/StandardMacros.IncrementInt` (`self.ForwardCurrentIndex`)
            (:`  `
              (goto _label)))
          (elif (>= _currentplaytime _output_starttime)
            (set `self.ForwardCurrentValue` _output_value)
            (else
              (set `self.ForwardCurrentValue` 0.0))))
        (else
          (set `self.ForwardCurrentValue` 0.0))))
    (:`then_1`
      (`Pawn.AddMovementInput` _ownercharacter (`Actor.GetActorForwardVector` _ownercharacter) (`self.ForwardCurrentValue`) false))))

(fn `ProcessInteractInput`
  (bind (_output_time _output_value) (break `/Game/Character/Blueprints/Clone/S_BoolInstruction` (`|GetArrayItem` (`self.InteractInstructions`) (`self.InteractCurrentIndex`))))
  (if (< (`self.InteractCurrentIndex`) (`KismetArrayLibrary.Array_Length` (`self.InteractInstructions`)))
    (if (>= (`self.CurrentPlayTime`) _output_time)
      (`|ExecutionSequence`
        (:`then_0`
          (for _array_element (`/Game/Character/Blueprints/Clone/BP_AlexClone.OverlappingInteractables` (`self.OwnerCharacter`))
            (if _output_value
              (`/Game/Environment/InteractiveObjects/I_PlayerInteractable.Interact` _array_element (`self.OwnerCharacter`))
              (else
                (`/Game/Environment/InteractiveObjects/I_PlayerInteractable.EndInteract` _array_element)))))
        (:`then_1`
          (`/Engine/EditorBlueprintResources/StandardMacros.IncrementInt` (`self.InteractCurrentIndex`)))))))

(fn `ProcessJumpInput`
  (bind _ownercharacter (`self.OwnerCharacter`))
  (bind (_output_time _output_value) (break `/Game/Character/Blueprints/Clone/S_BoolInstruction` (`|GetArrayItem` (`self.JumpInstructions`) (`self.JumpCurrentIndex`))))
  (if (< (`self.JumpCurrentIndex`) (`KismetArrayLibrary.Array_Length` (`self.JumpInstructions`)))
    (if (>= (`self.CurrentPlayTime`) _output_time)
      (`|ExecutionSequence`
        (:`then_0`
          (if _output_value
            (`Character.Jump` _ownercharacter)
            (else
              (`Character.StopJumping` _ownercharacter))))
        (:`then_1`
          (`/Engine/EditorBlueprintResources/StandardMacros.IncrementInt` (`self.JumpCurrentIndex`)))))))

(fn `ProcessLookInput`
  (locals (TargetPitch :type "Float (double-precision)") (TargetYaw :type "Float (double-precision)"))
  (bind _looksamples (`self.LookSamples`))
  (bind _lookcurrentindex (`self.LookCurrentIndex`))
  (bind _output (`|GetArrayItem` _looksamples _lookcurrentindex))
  (bind _output_time (break `/Game/Character/Blueprints/Clone/S_LookSample` (`|GetArrayItem` (`self.LookSamples`) (+ (`self.LookCurrentIndex`) 1))))
  (bind _output_2 (`|GetArrayItem` _looksamples (+ _lookcurrentindex 1)))
  (bind _returnvalue (`KismetMathLibrary.FClamp` (/ (- (`self.CurrentPlayTime`) (break `/Game/Character/Blueprints/Clone/S_LookSample` _output)) (- (break `/Game/Character/Blueprints/Clone/S_LookSample` _output_2) (break `/Game/Character/Blueprints/Clone/S_LookSample` _output)))))
  (if (< (+ (`self.LookCurrentIndex`) 1) (`KismetArrayLibrary.Array_Length` (`self.LookSamples`))) :!label _label
    (if (>= (`self.CurrentPlayTime`) _output_time)
      (`/Engine/EditorBlueprintResources/StandardMacros.IncrementInt` (`self.LookCurrentIndex`)
        (:`  `
          (goto _label)))
      (else
        _)))
  (if (< (`self.LookCurrentIndex`) (`KismetArrayLibrary.Array_Length` (`self.LookSamples`)))
    (`|ExecutionSequence`
      (:`then_0`
        (if (< (+ (`self.LookCurrentIndex`) 1) (`KismetArrayLibrary.Array_Length` (`self.LookSamples`)))
          (set `local.TargetPitch` (`KismetMathLibrary.Lerp` (`.Y` (`KismetMathLibrary.BreakVector2D` (`.Look_6_A7A837EF49D22DE4ADFA90BA32FA50B3` (break `/Game/Character/Blueprints/Clone/S_LookSample` _output)))) (`.Y` (`KismetMathLibrary.BreakVector2D` (`.Look_6_A7A837EF49D22DE4ADFA90BA32FA50B3` (break `/Game/Character/Blueprints/Clone/S_LookSample` _output_2)))) _returnvalue))
          (set `local.TargetYaw` (+ (`KismetMathLibrary.BreakVector2D` (`.Look_6_A7A837EF49D22DE4ADFA90BA32FA50B3` (break `/Game/Character/Blueprints/Clone/S_LookSample` _output))) (* _returnvalue (`KismetMathLibrary.NormalizeToRange` (- (`KismetMathLibrary.BreakVector2D` (`.Look_6_A7A837EF49D22DE4ADFA90BA32FA50B3` (break `/Game/Character/Blueprints/Clone/S_LookSample` _output_2))) (`KismetMathLibrary.BreakVector2D` (`.Look_6_A7A837EF49D22DE4ADFA90BA32FA50B3` (break `/Game/Character/Blueprints/Clone/S_LookSample` _output)))) -180.0 180.0))))
          (else
            (set `local.TargetPitch` (`.Y` (`KismetMathLibrary.BreakVector2D` (`.Look_6_A7A837EF49D22DE4ADFA90BA32FA50B3` (break `/Game/Character/Blueprints/Clone/S_LookSample` _output)))))
            (set `local.TargetYaw` (`KismetMathLibrary.BreakVector2D` (`.Look_6_A7A837EF49D22DE4ADFA90BA32FA50B3` (break `/Game/Character/Blueprints/Clone/S_LookSample` _output)))))))
      (:`then_1`
        (`Actor.K2_SetActorRotation` (`self.OwnerCharacter`) (`KismetMathLibrary.MakeRotator` 0.0 (`local.TargetPitch`) (`local.TargetYaw`)) false)))))

(fn `ProcessRightInput`
  (bind _currentplaytime (`self.CurrentPlayTime`))
  (bind _ownercharacter (`self.OwnerCharacter`))
  (bind (_output_starttime _output_endtime _output_value) (break `/Game/Character/Blueprints/Clone/S_MoveInstruction` (`|GetArrayItem` (`self.RightInstructions`) (`self.RightCurrentIndex`))))
  (`|ExecutionSequence`
    (:`then_0`
      (if (< (`self.RightCurrentIndex`) (`KismetArrayLibrary.Array_Length` (`self.RightInstructions`))) :!label _label
        (if (> _currentplaytime _output_endtime)
          (`/Engine/EditorBlueprintResources/StandardMacros.IncrementInt` (`self.RightCurrentIndex`)
            (:`  `
              (goto _label)))
          (elif (>= _currentplaytime _output_starttime)
            (set `self.RightCurrentValue` _output_value)
            (else
              (set `self.RightCurrentValue` 0.0))))
        (else
          (set `self.RightCurrentValue` 0.0))))
    (:`then_1`
      (`Pawn.AddMovementInput` _ownercharacter (`Actor.GetActorRightVector` _ownercharacter) (`self.RightCurrentValue`) false))))

(fn `ResetReplay`
  (bind (_starttransform_location _starttransform_rotation) (`KismetMathLibrary.BreakTransform` (`/Game/Character/Blueprints/Clone/BP_AlexClone.StartTransform` (`self.OwnerCharacter`))))
  (set `self.IsPlaying` false)
  (set `self.ForwardCurrentIndex` 0)
  (set `self.RightCurrentIndex` 0)
  (set `self.JumpCurrentIndex` 0)
  (set `self.InteractCurrentIndex` 0)
  (set `self.LookCurrentIndex` 0)
  (set `self.ForwardCurrentValue` 0.0)
  (set `self.RightCurrentValue` 0.0)
  (set `self.CurrentPlayTime` 0.0)
  (`Actor.K2_TeleportTo` (`self.OwnerCharacter`) _starttransform_location _starttransform_rotation))